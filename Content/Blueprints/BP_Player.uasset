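; BP_Player is an auto-running player character with jump and slide, using Enhanced Input.
; Tick constantly adds movement along world +X, as control yaw feeds only roll, and updates falling and grounded flags.
; Jump cancels the slide flag and, when grounded (stored as IsJumping), jumps after a short delay.
; Slide applies a strong downward impulse and sets a timed IsSliding flag, with DoOnce as a cooldown.
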(event Custom|Movement
  (Pawn|Input|AddMovementInput (Math|Vector|GetForwardVector (Math|Rotator|MakeRotator (.Yaw (Math|Rotator|BreakRotator (Pawn|GetControlRotation :!class /Script/Engine.Pawn))) 0.0 0.0)) 1.0 false))

(event Custom|Jumping%20Reset
  (Variables|Default|SetIsJumping (AI|Components|NavMovement|IsMovingonGround (Variables|Character|GetCharacterMovement))))

(event Custom|Check%20If%20Falling
  (if (and (AI|Components|NavMovement|IsFalling (Variables|Character|GetCharacterMovement)) (< (.z (Transformation|GetVelocity)) 0.0))
    (Variables|Default|SetIsFalling true)
    (else
      (Variables|Default|SetIsFalling false))))

(event Input|EnhancedActionEvents|EnhancedInputActionJump_IA
  (params (ActionValue :type Boolean) (ElapsedSeconds :type Float%20%28double-precision%29) (TriggeredSeconds :type Float%20%28double-precision%29) (InputAction :type Input%20Action%20Object%20Reference :default "/Game/Blueprints/Jump_IA.Jump_IA"))
  (Variables|Default|SetIsSliding false)
  (if (Variables|Default|GetIsJumping)
    (Utilities|FlowControl|Delay 0.2)
    (Character|Jump)))

(event Input|EnhancedActionEvents|EnhancedInputActionSlide_IA
  (params (ActionValue :type Boolean) (ElapsedSeconds :type Float%20%28double-precision%29) (TriggeredSeconds :type Float%20%28double-precision%29) (InputAction :type Input%20Action%20Object%20Reference :default "/Game/Blueprints/Slide_IA.Slide_IA"))
  (Utilities|FlowControl|DoOnce false :!label _label
    (:Completed
      (if (not (Variables|Default|GetIsSliding))
        (Physics|AddImpulse (Variables|Character|GetCharacterMovement) "0.000000,0.000000,-10000.000000" true)
        (Variables|Default|SetIsSliding true)
        (Utilities|FlowControl|Delay 1.0)
        (Variables|Default|SetIsSliding false)
        (Utilities|FlowControl|Delay 0.2)
        (goto _label Reset)))))

(event EventBeginPlay
  (bind _asplayer_controller (Utilities|Casting|CastToPlayerController (Pawn|GetController)))
  (Utilities|IsValid (PlayerController|LocalPlayerSubsystems|GetEnhancedInputLocalPlayerSubsystem _asplayer_controller)
    (:Is%20Valid
      (Input|AddMappingContext (PlayerController|LocalPlayerSubsystems|GetEnhancedInputLocalPlayerSubsystem _asplayer_controller) "/Game/Blueprints/IMC_Player.IMC_Player" 0 "(bIgnoreAllPressedKeysUntilRelease=True,bForceImmediately=False,bNotifyUserSettings=False)"))))

(event EventTick
  (params (DeltaSeconds :type Float%20%28single-precision%29))
  (CallFunction|Movement)
  (CallFunction|JumpingReset)
  (CallFunction|CheckifFalling))

(fn ConstructionScript)