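; Player Blueprint for a three-lane runner that constantly moves forward, with jump, slide and lane switching through Enhanced Input.
; Left and right inputs pick a clamped lane, and a shared Timeline lerps the Y position to it.
; Jump requires ground contact, while slide applies a downward impulse and holds a timed flag with a cooldown.
; Tick drives movement and a delayed, uncapped walk-speed increase, printed for debugging.
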(event Custom|Movement
  (Pawn|Input|AddMovementInput (Math|Vector|GetForwardVector (Math|Rotator|MakeRotator (.Yaw (Math|Rotator|BreakRotator (Pawn|GetControlRotation :!class /Script/Engine.Pawn))) 0.0 0.0)) 1.0 false))

(event Custom|Jumping%20Reset
  (Variables|Default|SetIsJumping (AI|Components|NavMovement|IsMovingonGround (Variables|Character|GetCharacterMovement))))

(event Custom|Increase%20Player%20Speed
  (bind _charactermovement (Variables|Character|GetCharacterMovement))
  (if true
    (Utilities|FlowControl|Delay 0.5)
    (bind _output_get (Variables|/Script/Engine.CharacterMovementComponent|SetMaxWalkSpeed _charactermovement (+ (Variables|/Script/Engine.CharacterMovementComponent|GetMaxWalkSpeed _charactermovement) (Variables|Default|GetSpeedIncreaseRate))))
    (Development|PrintString (Utilities|String|ToString(Float) _output_get))))

(event Input|EnhancedActionEvents|EnhancedInputActionJump_IA
  (params (ActionValue :type Boolean) (ElapsedSeconds :type Float%20%28double-precision%29) (TriggeredSeconds :type Float%20%28double-precision%29) (InputAction :type Input%20Action%20Object%20Reference :default "/Game/Blueprints/Player/inputs/Jump_IA.Jump_IA"))
  (Variables|Default|SetIsSliding false)
  (if (Variables|Default|GetIsJumping)
    (Utilities|FlowControl|Delay 0.2)
    (Character|Jump)))

(event Input|EnhancedActionEvents|EnhancedInputActionSlide_IA
  (params (ActionValue :type Boolean) (ElapsedSeconds :type Float%20%28double-precision%29) (TriggeredSeconds :type Float%20%28double-precision%29) (InputAction :type Input%20Action%20Object%20Reference :default "/Game/Blueprints/Player/inputs/Slide_IA.Slide_IA"))
  (Utilities|FlowControl|Sequence
    (:then_0
      (Utilities|FlowControl|DoOnce false :!label _label
        (:Completed
          (if (not (Variables|Default|GetIsSliding))
            (Physics|AddImpulse (Variables|Character|GetCharacterMovement) "0.000000,0.000000,-10000.000000" true)
            (Variables|Default|SetIsSliding true)
            (Utilities|FlowControl|Delay 1.0)
            (Variables|Default|SetIsSliding false)
            (Utilities|FlowControl|Delay 0.4)
            (goto _label Reset)))))))

(event EventBeginPlay
  (bind _asplayer_controller (Utilities|Casting|CastToPlayerController (Pawn|GetController)))
  (Utilities|IsValid (PlayerController|LocalPlayerSubsystems|GetEnhancedInputLocalPlayerSubsystem _asplayer_controller)
    (:Is%20Valid
      (Input|AddMappingContext (PlayerController|LocalPlayerSubsystems|GetEnhancedInputLocalPlayerSubsystem _asplayer_controller) "/Game/Blueprints/Player/inputs/IMC_Player.IMC_Player" 0 "(bIgnoreAllPressedKeysUntilRelease=True,bForceImmediately=False,bNotifyUserSettings=False)"))))

(event EventTick
  (params (DeltaSeconds :type Float%20%28single-precision%29))
  (Variables|Default|SetDelta%20Seconds DeltaSeconds)
  (CallFunction|Movement)
  (CallFunction|JumpingReset)
  (CallFunction|IncreasePlayerSpeed))

(event Input|ActionEvents|InputActionRight
  (params (Key :type Key%20Structure :default "None"))
  (bind _capsulecomponent (Variables|Collision|GetCapsuleComponent))
  (bind _lane_y (Variables|Default|GetLane%20Y))
  (bind _returnvalue (Transformation|GetWorldLocation _capsulecomponent))
  (:Pressed
    (Variables|Default|SetNewLane (Math|Integer|Clamp(Integer) (+ (Variables|Default|GetLane%20) 1) 0 2))
    (bind _newtrack_0 (Timeline|Timeline PlayFromStart)
      (:Update
        (Transformation|SetActorLocation (Math|Vector|MakeVector (.x _returnvalue) (Math|Float|Lerp (Utilities|Array|Get(acopy) _lane_y (Variables|Default|GetLane%20)) (Utilities|Array|Get(acopy) _lane_y (Variables|Default|GetNewLane)) _newtrack_0) (.z _returnvalue)) false false))
      (:Finished
        (Variables|Default|SetLane%20 (Variables|Default|GetNewLane))))))

(event Input|ActionEvents|InputActionLeft
  (params (Key :type Key%20Structure :default "None"))
  (bind _capsulecomponent (Variables|Collision|GetCapsuleComponent))
  (bind _lane_y (Variables|Default|GetLane%20Y))
  (bind _returnvalue (Transformation|GetWorldLocation _capsulecomponent))
  (:Pressed
    (Variables|Default|SetNewLane (Math|Integer|Clamp(Integer) (+ (Variables|Default|GetLane%20) -1) 0 2))
    (bind _newtrack_0 (Timeline|Timeline PlayFromStart)
      (:Update
        (Transformation|SetActorLocation (Math|Vector|MakeVector (.x _returnvalue) (Math|Float|Lerp (Utilities|Array|Get(acopy) _lane_y (Variables|Default|GetLane%20)) (Utilities|Array|Get(acopy) _lane_y (Variables|Default|GetNewLane)) _newtrack_0) (.z _returnvalue)) false false))
      (:Finished
        (Variables|Default|SetLane%20 (Variables|Default|GetNewLane))))))

(fn ConstructionScript)