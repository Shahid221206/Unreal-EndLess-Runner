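; BP_Magnet is a magnet powerup pickup that switches on the player's IsMagnetActive flag for a timed period.
; On box overlap with BP_Player it plays a sound and hides itself, then, if no magnet is active, sets the flag.
; After a MagnetTimer delay it clears the flag and destroys itself; a pickup during an active magnet only stays hidden.
; The box also destroys overlapping BP_Obstacle_Child_1 and BP_Obstacle_Child_2 actors.
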(event OnComponentBeginOverlap(Box)
  (params (OverlappedComponent :type Primitive%20Component%20Object%20Reference) (OtherActor :type Actor%20Object%20Reference) (OtherComp :type Primitive%20Component%20Object%20Reference) (OtherBodyIndex :type Integer) (bFromSweep :type Boolean) (SweepResult :type Hit%20Result%20Structure%20%28by%20ref%29))
  (Utilities|FlowControl|Sequence
    (:then_0
      (bind _asbp_player (Utilities|Casting|CastToBP_Player OtherActor))
      (Audio|PlaySound2D "/Game/StarterContent/Audio/Explosion01.Explosion01" 1.0 1.0 0.0 0 0)
      (Rendering|SetActorHiddenInGame true)
      (if (not (Variables|/Game/Blueprint/Player/BP_Player.BP_Player_C|GetIsMagnetActive? _asbp_player))
        (Variables|/Game/Blueprint/Player/BP_Player.BP_Player_C|SetIsMagnetActive? _asbp_player true)
        (Utilities|FlowControl|Delay (Variables|Default|GetMagnetTimer))
        (bind _returnvalue (Actor|GetActorOfClass "/Game/Blueprint/Player/BP_Player.BP_Player_C"))
        (Utilities|IsValid _returnvalue
          (:Is%20Valid
            (Variables|/Game/Blueprint/Player/BP_Player.BP_Player_C|SetIsMagnetActive? _returnvalue false)
            (Actor|DestroyActor)))))
    (:then_1
      (bind _asbp_obstacle_child_1 (Utilities|Casting|CastToBP_Obstacle_Child_1 OtherActor))
      (Actor|DestroyActor _asbp_obstacle_child_1))
    (:then_2
      (bind _asbp_obstacle_child_2 (Utilities|Casting|CastToBP_Obstacle_Child_2 OtherActor))
      (Actor|DestroyActor _asbp_obstacle_child_2))))

(event EventBeginPlay)

(event Collision|EventActorBeginOverlap
  (params (OtherActor :type Actor%20Object%20Reference)))

(event EventTick
  (params (DeltaSeconds :type Float%20%28single-precision%29)))

(fn ConstructionScript)