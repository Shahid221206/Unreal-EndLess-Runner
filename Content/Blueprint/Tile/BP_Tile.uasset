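; Floor tile for an endless runner that randomly places obstacles and coins across its lanes.
; The construction script creates arrow-marked spawn points per lane, shuffles them, and adds a few obstacles and coins as child actors.
; When the player overlaps the tile's box, it tells GM_EndlessRuneer to extend the floor and increments the score.
; GetAttachPoint exposes the Arrow transform as an attach point.
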(event OnComponentBeginOverlap(Box)
  (params (OverlappedComponent :type Primitive%20Component%20Object%20Reference) (OtherActor :type Actor%20Object%20Reference) (OtherComp :type Primitive%20Component%20Object%20Reference) (OtherBodyIndex :type Integer) (bFromSweep :type Boolean) (SweepResult :type Hit%20Result%20Structure%20%28by%20ref%29))
  (Utilities|Casting|CastToBP_Player OtherActor)
  (Utilities|FlowControl|Sequence
    (:then_0
      (bind _asgm_endless_runeer (Utilities|Casting|CastToGM_EndlessRuneer (Game|GetGameMode)))
      (Default|ExtendFloor _asgm_endless_runeer)
      (bind _result (Math|Float|IncrementFloat (Variables|/Game/Game_Mode/GM_EndlessRuneer.GM_EndlessRuneer_C|GetCurrentScore _asgm_endless_runeer))
        (:%20%20
          (Variables|/Game/Game_Mode/GM_EndlessRuneer.GM_EndlessRuneer_C|SetCurrentScore _asgm_endless_runeer _result))))))

(event EventBeginPlay)

(event Collision|EventActorBeginOverlap
  (params (OtherActor :type Actor%20Object%20Reference)))

(event EventTick
  (params (DeltaSeconds :type Float%20%28single-precision%29)))

(fn ConstructionScript
  (CallFunction|SetupSpawnPoint)
  (CallFunction|SpawnObstacles)
  (CallFunction|CoinSpawnPoint)
  (CallFunction|SpawnCoins))

(fn GetAttachPoint
  (return (Transformation|GetWorldTransform (Variables|Default|GetArrow))))

(fn SetupSpawnPoint
  (for _array_element (Variables|Default|GetLane%20Y)
    (for _index (range 0 0)
      (bind _returnvalue (AddComponent|AddArrowComponent false (Math|Transform|MakeTransform (Math|Vector|MakeVector (* _index 5.2e+02) _array_element 0.0))))
      (Utilities|Array|Add (Variables|Default|GetSpawnPoints) (Transformation|GetWorldTransform _returnvalue)))))

(fn SpawnObstacles
  (bind _output_get (LocalVariables|SetRandomSpawnPoint (Variables|Default|GetSpawnPoints)))
  (Utilities|Array|Shuffle _output_get)
  (for _index (range 0 (Math|Random|RandomIntegerinRange 0 1))
    (switch int (Math|Random|RandomIntegerinRange 0 1)
      (:0
        (AddComponent|AddChildActorComponent false (Math|Transform|MakeRelativeTransform (Utilities|Array|Get(acopy) (LocalVariables|GetRandomSpawnPoint) _index) (Transformation|GetActorTransform))))
      (:1
        (AddComponent|AddChildActorComponent false (Math|Transform|MakeRelativeTransform (Utilities|Array|Get(acopy) (LocalVariables|GetRandomSpawnPoint) _index) (Transformation|GetActorTransform)))))))

(fn CoinSpawnPoint
  (for _array_element (Variables|Default|GetLane%20Y)
    (for _index (range 0 4)
      (bind _returnvalue (AddComponent|AddArrowComponent false (Math|Transform|MakeTransform (Math|Vector|MakeVector (* _index 2e+02) _array_element 0.0))))
      (Components|Arrow|SetArrowColor(LinearColor) _returnvalue "(R=1.000000,G=0.776968,B=0.000000,A=1.000000)")
      (Utilities|Array|Add (Variables|Default|GetCoinSpawnPoints) (Transformation|GetWorldTransform _returnvalue)))))

(fn SpawnCoins
  (bind _output_get (LocalVariables|SetRandomSpawnPoint (Variables|Default|GetCoinSpawnPoints)))
  (Utilities|Array|Shuffle _output_get)
  (for _index (range 0 (Math|Random|RandomIntegerinRange 0 3))
    (switch int 0
      (:0
        (AddComponent|AddChildActorComponent false (Math|Transform|MakeRelativeTransform (Utilities|Array|Get(acopy) (LocalVariables|GetRandomSpawnPoint) _index) (Transformation|GetActorTransform)))))))