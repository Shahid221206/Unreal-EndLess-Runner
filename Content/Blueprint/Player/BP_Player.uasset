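; Player character for a three-lane endless runner that runs forward automatically while its walk speed ramps up toward a limit.
; Left and right inputs lerp Y between lanes on a Timeline; jump requires ground contact.
; Slide slams the character down and briefly ignores the Destructible collision channel, gated by a cooldown.
; Death ragdolls the mesh, shows the game-over widget and saves the GameMode score when it sets a high score.
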(event Custom|Movement
  (Pawn|Input|AddMovementInput (Math|Vector|GetForwardVector (Math|Rotator|MakeRotator (.Yaw (Math|Rotator|BreakRotator (Pawn|GetControlRotation :!class /Script/Engine.Pawn))) 0.0 0.0)) 1.0 false))

(event Custom|Jumping%20Reset
  (Variables|Default|SetIsJumping (AI|Components|NavMovement|IsMovingonGround (Variables|Character|GetCharacterMovement))))

(event Custom|Increase%20Player%20Speed
  (bind _charactermovement (Variables|Character|GetCharacterMovement))
  (if (not (== (Variables|/Script/Engine.CharacterMovementComponent|GetMaxWalkSpeed _charactermovement) (Variables|Default|GetSpeedLimit)))
    (Utilities|FlowControl|Delay 0.5)
    (Variables|/Script/Engine.CharacterMovementComponent|SetMaxWalkSpeed _charactermovement (+ (Variables|/Script/Engine.CharacterMovementComponent|GetMaxWalkSpeed _charactermovement) (Variables|Default|GetSpeedIncreaseRate)))))

(event EventBeginPlay
  (bind _returnvalue (UserInterface|CreateWidget "/Game/Blueprint/UI/WB_Player_Interface.WB_Player_Interface_C"))
  (Variables|/Script/Engine.PlayerController|SetbShowMouseCursor (Game|GetPlayerController 0) true)
  (UserInterface|Viewport|AddtoViewport _returnvalue 0))

(event Collision|EventActorBeginOverlap
  (params (OtherActor :type Actor%20Object%20Reference)))

(event EventTick
  (params (DeltaSeconds :type Float%20%28single-precision%29))
  (Variables|Default|SetDelta%20Seconds DeltaSeconds)
  (CallFunction|Movement)
  (CallFunction|JumpingReset)
  (CallFunction|IncreasePlayerSpeed))

(event Input|ActionEvents|InputActionRight
  (params (Key :type Key%20Structure :default "None"))
  (bind _capsulecomponent (Variables|Collision|GetCapsuleComponent))
  (bind _lane_y (Variables|Default|GetLane%20Y))
  (bind _returnvalue (Transformation|GetWorldLocation _capsulecomponent))
  (:Pressed
    (Variables|Default|SetNewLane (Math|Integer|Clamp(Integer) (+ (Variables|Default|GetLane%20) 1) 0 2))
    (bind _newtrack_0 (Timeline|Timeline PlayFromStart)
      (:Update
        (Transformation|SetActorLocation (Math|Vector|MakeVector (.x _returnvalue) (Math|Float|Lerp (Utilities|Array|Get(acopy) _lane_y (Variables|Default|GetLane%20)) (Utilities|Array|Get(acopy) _lane_y (Variables|Default|GetNewLane)) _newtrack_0) (.z _returnvalue)) false false))
      (:Finished
        (Variables|Default|SetLane%20 (Variables|Default|GetNewLane))))))

(event Input|ActionEvents|InputActionLeft
  (params (Key :type Key%20Structure :default "None"))
  (bind _capsulecomponent (Variables|Collision|GetCapsuleComponent))
  (bind _lane_y (Variables|Default|GetLane%20Y))
  (bind _returnvalue (Transformation|GetWorldLocation _capsulecomponent))
  (:Pressed
    (Variables|Default|SetNewLane (Math|Integer|Clamp(Integer) (+ (Variables|Default|GetLane%20) -1) 0 2))
    (bind _newtrack_0 (Timeline|Timeline PlayFromStart)
      (:Update
        (Transformation|SetActorLocation (Math|Vector|MakeVector (.x _returnvalue) (Math|Float|Lerp (Utilities|Array|Get(acopy) _lane_y (Variables|Default|GetLane%20)) (Utilities|Array|Get(acopy) _lane_y (Variables|Default|GetNewLane)) _newtrack_0) (.z _returnvalue)) false false))
      (:Finished
        (Variables|Default|SetLane%20 (Variables|Default|GetNewLane))))))

(event Input|ActionEvents|InputActionJump
  (params (Key :type Key%20Structure :default "None"))
  (:Pressed
    (Variables|Default|SetIsSliding false)
    (if (Variables|Default|GetIsJumping)
      (Utilities|FlowControl|Delay 0.2)
      (Character|Jump))))

(event Input|ActionEvents|InputActionSlide
  (params (Key :type Key%20Structure :default "None"))
  (bind _capsulecomponent (Variables|Collision|GetCapsuleComponent))
  (:Pressed
    (Utilities|FlowControl|DoOnce false :!label _label
      (:Completed
        (if (not (Variables|Default|GetIsSliding))
          (Physics|AddImpulse (Variables|Character|GetCharacterMovement) "0.000000,0.000000,-10000.000000" true)
          (Variables|Default|SetIsSliding true)
          (Collision|SetCollisionResponsetoChannel _capsulecomponent "ECC_Destructible" "ECR_Ignore")
          (Utilities|FlowControl|Delay 1.0)
          (Variables|Default|SetIsSliding false)
          (Collision|SetCollisionResponsetoChannel _capsulecomponent "ECC_Destructible" "ECR_Block")
          (Utilities|FlowControl|Delay 0.4)
          (goto _label Reset))))))

(fn ConstructionScript)

(fn Death
  (Pawn|Components|CharacterMovement|DisableMovement (Variables|Character|GetCharacterMovement))
  (Input|DisableInput 0)
  (Physics|SetSimulatePhysics (Variables|Character|GetMesh) true)
  (Viewport|RemoveAllWidgets)
  (bind _returnvalue (UserInterface|CreateWidget "/Game/Blueprint/UI/WB_GameOver.WB_GameOver_C"))
  (UserInterface|Viewport|AddtoViewport _returnvalue 0)
  (Variables|/Script/Engine.PlayerController|SetbShowMouseCursor (Game|GetPlayerController 0) true)
  (bind _asgm_endless_runeer (Utilities|Casting|CastToGM_EndlessRuneer (Game|GetGameMode)))
  (bind _returnvalue_2 (SaveGame|DoesSaveGameExist "HighScore"))
  (if _returnvalue_2
    (bind _returnvalue_3 (SaveGame|LoadGamefromSlot "HighScore"))
    (bind _output_get (Variables|Default|SetSaverSubClass _returnvalue_3))
    (bind _asbp_save_game (Utilities|Casting|CastToBP_Save_Game _output_get)
      (:then
        (if (> (Variables|/Game/Game_Mode/GM_EndlessRuneer.GM_EndlessRuneer_C|GetCurrent%20Score _asgm_endless_runeer) (Variables|/Game/Blueprint/SaveGame/BP_Save_Game.BP_Save_Game_C|GetHighScore _asbp_save_game))
          (Variables|/Game/Blueprint/SaveGame/BP_Save_Game.BP_Save_Game_C|SetHighScore _asbp_save_game (Variables|/Game/Game_Mode/GM_EndlessRuneer.GM_EndlessRuneer_C|GetCurrent%20Score _asgm_endless_runeer))
          (SaveGame|SaveGametoSlot (Variables|Default|GetSaverSubClass) "HighScore")))
      (:CastFailed
        (Development|PrintString "Hello")))
    (else
      (bind _returnvalue_4 (SaveGame|CreateSaveGameObject "/Game/Blueprint/SaveGame/BP_Save_Game.BP_Save_Game_C"))
      (bind _output_get_2 (Variables|Default|SetSaverSubClass _returnvalue_4))
      (bind _asbp_save_game_2 (Utilities|Casting|CastToBP_Save_Game _output_get_2))
      (Variables|/Game/Blueprint/SaveGame/BP_Save_Game.BP_Save_Game_C|SetHighScore _asbp_save_game_2 (Variables|/Game/Game_Mode/GM_EndlessRuneer.GM_EndlessRuneer_C|GetCurrent%20Score _asgm_endless_runeer))
      (SaveGame|SaveGametoSlot (Variables|Default|GetSaverSubClass) "HighScore"))))