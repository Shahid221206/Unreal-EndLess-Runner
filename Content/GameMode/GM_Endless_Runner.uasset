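; Endless runner game mode that builds and recycles a floor from three road tile types.
; AddFloor spawns the type chosen by TileSelector at FloorAttachPoint, then advances that point to the new tile's attach point.
; TileSelector rerolls every Tick, so the BeginPlay batch shares one type.
; ExtendFloor adds a tile and destroys the oldest in any per-type array exceeding NumberOfTiles plus a margin.
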(event Custom|Tile%20Selector
  (Variables|Default|SetTileSelector (Math|Random|RandomIntegerinRange 0 2)))

(event EventBeginPlay
  (for _index (range 0 (- (Variables|Default|GetNumberOfTiles) 1))
    (CallFunction|AddFloor)))

(event EventTick
  (params (DeltaSeconds :type Float%20%28single-precision%29))
  (CallFunction|TileSelector))

(fn ConstructionScript)

(fn AddFloor
  (bind _tileselector (Variables|Default|GetTileSelector))
  (Utilities|FlowControl|Sequence
    (:then_0
      (if (== _tileselector 0)
        (bind _returnvalue (Game|SpawnActorfromClass "/Game/Blueprints/Tiles/BP_Tiles_Road_1.BP_Tiles_Road_1_C" (Variables|Default|GetFloorAttachPoint) "Undefined" "MultiplyWithRoot" 0 0))
        (bind _returnvalue_2 (Default|GetAttachPoint _returnvalue))
        (Variables|Default|SetFloorAttachPoint _returnvalue_2)
        (Utilities|Array|Add (Variables|Default|GetFloorTiles1) _returnvalue)))
    (:then_1
      (if (== _tileselector 1)
        (bind _returnvalue_3 (Game|SpawnActorfromClass "/Game/Blueprints/Tiles/BP_Tiles_Road_2.BP_Tiles_Road_2_C" (Variables|Default|GetFloorAttachPoint) "Undefined" "MultiplyWithRoot" 0 0))
        (bind _returnvalue_4 (Default|GetAttachPoint _returnvalue_3))
        (Variables|Default|SetFloorAttachPoint _returnvalue_4)
        (Utilities|Array|Add (Variables|Default|GetFloorTiles2) _returnvalue_3)))
    (:then_2
      (if (== _tileselector 2)
        (bind _returnvalue_5 (Game|SpawnActorfromClass "/Game/Blueprints/Tiles/BP_Tiles_Road_3.BP_Tiles_Road_3_C" (Variables|Default|GetFloorAttachPoint) "Undefined" "MultiplyWithRoot" 0 0))
        (Development|PrintString "Hello")
        (bind _returnvalue_6 (Default|GetAttachPoint _returnvalue_5))
        (Variables|Default|SetFloorAttachPoint _returnvalue_6)
        (Utilities|Array|Add (Variables|Default|GetFloorTile3) _returnvalue_5)))))

(fn ExtendFloor
  (bind _floortiles1 (Variables|Default|GetFloorTiles1))
  (bind _floortiles2 (Variables|Default|GetFloorTiles2))
  (bind _floortile3 (Variables|Default|GetFloorTile3))
  (bind _output (Utilities|Array|Get(acopy) _floortiles1))
  (bind _output_2 (Utilities|Array|Get(acopy) _floortiles2))
  (bind _output_3 (Utilities|Array|Get(acopy) _floortile3))
  (CallFunction|AddFloor)
  (Utilities|FlowControl|Sequence
    (:then_0
      (if (> (Utilities|Array|Length (Variables|Default|GetFloorTiles1)) (+ (Variables|Default|GetNumberOfTiles) 3))
        (Actor|DestroyActor _output)
        (Utilities|Array|RemoveItem _floortiles1 _output)))
    (:then_1
      (if (> (Utilities|Array|Length (Variables|Default|GetFloorTiles2)) (+ (Variables|Default|GetNumberOfTiles) 3))
        (Actor|DestroyActor _output_2)
        (Utilities|Array|RemoveItem _floortiles2 _output_2)))
    (:then_2
      (if (> (Utilities|Array|Length (Variables|Default|GetFloorTile3)) (+ (Variables|Default|GetNumberOfTiles) 3))
        (Actor|DestroyActor _output_3)
        (Utilities|Array|RemoveItem _floortile3 _output_3)))))