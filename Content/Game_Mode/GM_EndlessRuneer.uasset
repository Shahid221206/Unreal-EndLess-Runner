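; Game mode for an endless runner that builds and recycles the floor from BP_Tile actors.
; On BeginPlay it spawns NumberOfTiles tiles, chaining each at the attach point returned by the previous one.
; ExtendFloor appends a tile and, once the tracked array exceeds NumberOfTiles plus a small buffer, destroys the oldest, keeping the track length bounded.
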(event EventBeginPlay
  (for _index (range 0 (- (Variables|Default|GetNumberOfTiles) 1))
    (CallFunction|AddFloor)))

(event EventTick
  (params (DeltaSeconds :type Float%20%28single-precision%29)))

(fn ConstructionScript)

(fn AddFloor
  (bind _returnvalue (Game|SpawnActorfromClass "/Game/Blueprint/Tile/BP_Tile.BP_Tile_C" (Variables|Default|GetFloorAttachPoint) "Undefined" "MultiplyWithRoot" 0 0))
  (bind _returnvalue_2 (Default|GetAttachPoint _returnvalue))
  (Variables|Default|SetFloorAttachPoint _returnvalue_2)
  (Utilities|Array|Add (Variables|Default|GetFloorTiles1) _returnvalue))

(fn ExtendFloor
  (bind _floortiles1 (Variables|Default|GetFloorTiles1))
  (bind _output (Utilities|Array|Get(acopy) _floortiles1))
  (CallFunction|AddFloor)
  (if (> (Utilities|Array|Length (Variables|Default|GetFloorTiles1)) (+ (Variables|Default|GetNumberOfTiles) 3))
    (Actor|DestroyActor _output)
    (Utilities|Array|RemoveItem _floortiles1 _output)))